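; BP_ChessPiece is a chess piece actor that holds its type, color, selection state and current square reference.
; Initialize sets color-based materials on the piece mesh and on an outline mesh that copies its static mesh.
; Moves and captures update square occupancy and trigger teleport or explode effects on the square, with capture destroying the actor.
; Promotion swaps the mesh and refreshes the outline, while moved and double-step flags track move history.
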(fn `ApplyMaterialBasedOnColor`
  (switch `/Game/Chess/Core/Engine/EColor` (`self.Color`)
    (:`NewEnumerator0`
      (`PrimitiveComponent.SetMaterial` (`self.StaticMesh_Piece`) 0 "/Game/Chess/Core/Pieces/MI_ChessPiece_White.MI_ChessPiece_White"))
    (:`NewEnumerator1`
      (`PrimitiveComponent.SetMaterial` (`self.StaticMesh_Piece`) 0 "/Game/Chess/Core/Pieces/MI_ChessPiece_Black.MI_ChessPiece_Black")))
  (return))

(fn `ClearCurrentSquare`
  (set `self.SquareReference` null)
  (return))

(fn `GetCurrentSquare`
  (returns (SquareReference :type "/Game/Chess/Core/Board/BP_Square Object Reference"))
  (return (`self.SquareReference`)))

(fn `GetEnPassantVaraible`
  (returns (bPawnMovedByTwoLastTurn :type Boolean))
  (return (`self.bPawnMovedByTwoLastTurn`)))

(fn `GetMovedThisGame`
  (returns (bMovedThisGame :type Boolean))
  (return (`self.bMovedThisGame`)))

(fn `GetPieceColor`
  (returns (Color :type "/Game/Chess/Core/Engine/EColor Enum"))
  (return (`self.Color`)))

(fn `GetPieceType`
  (returns (Type :type "/Game/Chess/Core/Pieces/EChessPiece Enum"))
  (return (`self.Type`)))

(fn `Initialize`
  (`self.ApplyMaterialBasedOnColor`)
  (`self.SetOutlineMesh`)
  (return))

(fn `IsCaptured`
  (`/Game/Chess/Core/Board/BP_Square.ActivateExplodeFX` (`self.SquareReference`))
  (`/Game/Chess/Core/Board/BP_Square.RemoveOccupant` (`self.SquareReference`))
  (set `self.SquareReference` null)
  (`self.K2_DestroyActor`)
  (return))

(fn `MoveToSquare`
  (params (Square :type "/Game/Chess/Core/Board/BP_Square Object Reference"))
  (`/Game/Chess/Core/Board/BP_Square.RemoveOccupant` (`self.SquareReference`))
  (bind _output_get (set `self.SquareReference` Square))
  (`self.K2_SetActorLocation` (`/Game/Chess/Core/Board/BP_Square.GetSquareWorldLocation` _output_get) true)
  (`/Game/Chess/Core/Board/BP_Square.ActivateTeleportFX` (`self.SquareReference`))
  (`/Game/Chess/Core/Board/BP_Square.SetOccupant` (`self.SquareReference`) self)
  (set `self.bMovedThisGame` true)
  (return))

(fn `Promote`
  (params (Type :type "/Game/Chess/Core/Pieces/EChessPiece Enum" :default "NewEnumerator0"))
  (bind _output_get (set `self.Type` Type))
  (switch `/Game/Chess/Core/Pieces/EChessPiece` _output_get
    (:`NewEnumerator1`
      (`StaticMeshComponent.SetStaticMesh` (`self.StaticMesh_Piece`) "/Game/Chess/Core/Pieces/S_Knight.S_Knight"))
    (:`NewEnumerator2`
      (`StaticMeshComponent.SetStaticMesh` (`self.StaticMesh_Piece`) "/Game/Chess/Core/Pieces/S_Bishop.S_Bishop"))
    (:`NewEnumerator3`
      (`StaticMeshComponent.SetStaticMesh` (`self.StaticMesh_Piece`) "/Game/Chess/Core/Pieces/S_Rook.S_Rook"))
    (:`NewEnumerator4`
      (`StaticMeshComponent.SetStaticMesh` (`self.StaticMesh_Piece`) "/Game/Chess/Core/Pieces/S_Queen.S_Queen")))
  (`self.SetOutlineMesh`)
  (return))

(fn `SelectPiece`
  (set `self.bSelected` true)
  (`/Game/Chess/Core/Board/BP_Square.SelectOccupant` (`self.SquareReference`))
  (return))

(fn `SetColor`
  (params (Color :type "/Game/Chess/Core/Engine/EColor Enum" :default "NewEnumerator0"))
  (set `self.Color` Color)
  (return))

(fn `SetCurrentSquare`
  (params (NewSquare :type "/Game/Chess/Core/Board/BP_Square Object Reference"))
  (set `self.SquareReference` NewSquare)
  (return))

(fn `SetEnPassantVaraible`
  (params (PawnMovedByTwo :type Boolean))
  (set `self.bPawnMovedByTwoLastTurn` PawnMovedByTwo)
  (return))

(fn `SetOutlineMesh`
  (`StaticMeshComponent.SetStaticMesh` (`self.StaticMesh_Outline`) (`StaticMeshComponent.StaticMesh` (`self.StaticMesh_Piece`)))
  (switch `/Game/Chess/Core/Engine/EColor` (`self.Color`)
    (:`NewEnumerator0`
      (`PrimitiveComponent.SetMaterial` (`self.StaticMesh_Outline`) 0 "/Game/Chess/Core/Pieces/MI_ChessPiece_Outline_White.MI_ChessPiece_Outline_White"))
    (:`NewEnumerator1`
      (`PrimitiveComponent.SetMaterial` (`self.StaticMesh_Outline`) 0 "/Game/Chess/Core/Pieces/MI_ChessPiece_Outline_Black.MI_ChessPiece_Outline_Black")))
  (return))

(fn `UnselectPiece`
  (set `self.bSelected` false)
  (return))

(fn `UserConstructionScript`)