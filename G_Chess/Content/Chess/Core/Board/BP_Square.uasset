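; BP_Square is a single chessboard square that stores its coordinates, algebraic notation, color and occupying piece.
; Boolean state flags drive one marker mesh's material and visibility for highlight, selection, attack and selected-piece feedback.
; Highlighting flags the square attackable if occupied or if the game mode reports an en passant move.
; It binds to the board's reset event to clear markers, and exposes occupant color queries plus explosion and teleport effects.
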(event `InitEvent`
  ;[1 1 1] Initial event that binds the Reset Square event to Reset All Squares in the Chessboard BP
  (`/Engine/EditorBlueprintResources/StandardMacros.IsValid` (`self.BoardReference`)
    (:`Is Valid`
      (add `/Game/Chess/Core/Board/BP_ChessBoard.OnResetAllSquareMarkers` (`self.BoardReference`) (delegate `ResetSquare`)))))

(event `ResetSquare`
  ;[1 1 1] Resets the highlight markers for the square.
  (`self.ResetMarker`))

(fn `ActivateExplodeFX`
  (`ActorComponent.Activate` (`self.ParticleSystem_ExplodeFX`) true)
  (`AudioComponent.Play` (`self.Audio_Explosion`) 0.0)
  (return))

(fn `ActivateTeleportFX`
  (`ActorComponent.Activate` (`self.ParticleSystem_TeleportFX`) true)
  (return))

(fn `CanBeAttackedEnPassant`
  (returns (Attackable :type Boolean))
  (return (`/Game/Chess/Core/Engine/BP_GameMode_Core.IsMoveEnPassant` (`self.GameModeReference`) (`/Game/Chess/Core/Engine/BP_GameMode_Core.SelectedChessPieceReference` (`self.GameModeReference`)) self)))

(fn `GetAttackableStatus`
  (returns (bIsAttackable :type Boolean))
  (return (and (`self.bHighlighted`) (`self.bAttackable`))))

(fn `GetColumnLetterInNotation`
  (returns (ColumnLetter :type String))
  (switch `int` (`self.PositionX`)
    (:`1`
      (return "a"))
    (:`2`
      (return "b"))
    (:`3`
      (return "c"))
    (:`4`
      (return "d"))
    (:`5`
      (return "e"))
    (:`6`
      (return "f"))
    (:`7`
      (return "g"))
    (:`8`
      (return "h"))))

(fn `GetNotation`
  (returns (Notation :type String))
  (return (`self.Notation`)))

(fn `GetOccupant`
  (returns (Occupant :type "/Game/Chess/Core/Pieces/BP_ChessPiece Object Reference"))
  (return (`self.OccupantReference`)))

(fn `GetSquareColor`
  (returns (Color :type "/Game/Chess/Core/Engine/EColor Enum"))
  (return (`self.Color`)))

(fn `GetSquareCoordinates`
  (returns (PositionX :type Integer) (PositionY :type Integer))
  (return (`self.PositionX`) (`self.PositionY`)))

(fn `GetSquareWorldLocation`
  (returns (Location :type "Vector Structure"))
  (return (`SceneComponent.K2_GetComponentLocation` (`self.Billboard`))))

(fn `HasAnOccupant`
  (returns (bHasOccupant :type Boolean))
  (return (`KismetSystemLibrary.IsValid` (`self.OccupantReference`))))

(fn `HasAnOccupantOfColor`
  (params (Color :type "/Game/Chess/Core/Engine/EColor Enum" :default "NewEnumerator0"))
  (returns (HasOccupantOfColor :type Boolean))
  (if (`self.HasAnOccupant`)
    (return (`|EnumEquality` Color (`/Game/Chess/Core/Pieces/BP_ChessPiece.Color` (`self.GetOccupant`))))
    (else
      (return false))))

(fn `HasAnOccupantOfDifferentColor`
  (params (Piece :type "/Game/Chess/Core/Pieces/BP_ChessPiece Object Reference"))
  (returns (bHasEnemyPiece :type Boolean))
  (switch `/Game/Chess/Core/Engine/EColor` (`/Game/Chess/Core/Pieces/BP_ChessPiece.GetPieceColor` Piece)
    (:`NewEnumerator0`
      (if (`self.HasAnOccupantOfColor` "NewEnumerator1")
        (return true)
        (else
          (return false))))
    (:`NewEnumerator1`
      (if (`self.HasAnOccupantOfColor` "NewEnumerator0")
        (return true)
        (else
          (return false))))))

(fn `HasAnOccupantOfTheSameColor`
  (params (Piece :type "/Game/Chess/Core/Pieces/BP_ChessPiece Object Reference"))
  (returns (bHasEnemyPiece :type Boolean))
  (return (`self.HasAnOccupantOfColor` (`/Game/Chess/Core/Pieces/BP_ChessPiece.GetPieceColor` Piece))))

(fn `HighlightMarker`
  (`|ExecutionSequence`
    (:`then_0`
      ;[0.1041 0.9901 1] Set flags to HIGHLIGHTED only
      (set `self.bHighlighted` true)
      (set `self.bSelected` false)
      (set `self.bAttackable` false)
      (set `self.bChessPieceSelected` false))
    (:`then_1`
      ;[0.3485 0.2475 1] Check for Occupant
      (if (`self.HasAnOccupant`)
        (set `self.bAttackable` true :!label _label)
        (elif (`self.CanBeAttackedEnPassant`)
          (goto _label)
          (else
            _)))
      (`self.SetMarkerColor`))
    (:`then_2`
      (return))))

(fn `Initialize`
  (`self.SetPlayerControllerReference`)
  (`self.SetGameModeReference`)
  (`self.SetNotation`)
  (`self.InitEvent`)
  (return))

(fn `RemoveOccupant`
  (set `self.OccupantReference` null)
  (return))

(fn `ResetMarker`
  (`|ExecutionSequence`
    (:`then_0`
      (set `self.bHighlighted` false)
      (set `self.bSelected` false)
      (set `self.bAttackable` false)
      (set `self.bChessPieceSelected` false))
    (:`then_1`
      (`self.SetMarkerColor`) ; This is changing the MarkerVisible to False based on above conditions
      (return))))

(fn `SelectMarker`
  (if (`self.bHighlighted`)
    (set `self.bSelected` true)
    (`self.SetMarkerColor`)
    (return)
    (else
      (return))))

(fn `SelectOccupant`
  (`|ExecutionSequence`
    (:`then_0`
      ;[1 1 1] Unhighlight the square - a piece is selected, not the square
      (set `self.bAttackable` false)
      (set `self.bHighlighted` false)
      (set `self.bSelected` false))
    (:`then_1`
      ;[1 1 1] Highlight the selected Piece
      (if (`self.HasAnOccupant`)
        (set `self.bChessPieceSelected` true)
        (`self.SetMarkerColor`)
        (return)
        (else
          (return))))))

(fn `SetBoardReference`
  (params (Board :type "/Game/Chess/Core/Board/BP_ChessBoard Object Reference"))
  (set `self.BoardReference` Board)
  (return))

(fn `SetGameModeReference`
  (`/Engine/EditorBlueprintResources/StandardMacros.IsValid` (`self.GameModeReference`)
    (:`Is Valid`
      _)
    (:`Is Not Valid`
      (set `self.GameModeReference` (cast `/Game/Chess/Core/Engine/BP_GameMode_Core` (`GameplayStatics.GetGameMode`) :!pure true))))
  (return))

(fn `SetMarkerColor`
  (if (`self.bHighlighted`)
    (if (`self.bSelected`)
      (set `self.bMarkerVisible` true)
      (set `self.MarkerActiveMaterial` (`self.MarkerSelectMaterial`))
      (elif (`self.bAttackable`)
        (set `self.bMarkerVisible` true)
        (set `self.MarkerActiveMaterial` (`self.MarkerAttackMaterial`))
        (else
          (set `self.bMarkerVisible` true)
          (set `self.MarkerActiveMaterial` (`self.MarkerHighlightMaterial`)))))
    (elif (`self.bChessPieceSelected`)
      (set `self.bMarkerVisible` true)
      (set `self.MarkerActiveMaterial` (`self.MarkerChessPieceMaterial`))
      (else
        (set `self.bMarkerVisible` false)
        (set `self.MarkerActiveMaterial` (`self.MarkerHighlightMaterial`)))))
  (`PrimitiveComponent.SetMaterial` (`self.StaticMesh_Marker`) 0 (`self.MarkerActiveMaterial`))
  (`SceneComponent.SetVisibility` (`self.StaticMesh_Marker`) (`self.bMarkerVisible`) false)
  (return))

(fn `SetNotation`
  (set `self.Notation` (`KismetStringLibrary.Concat_StrStr` (`self.GetColumnLetterInNotation`) (`KismetStringLibrary.Conv_IntToString` (`self.PositionY`))))
  (return))

(fn `SetOccupant`
  (params (Piece :type "/Game/Chess/Core/Pieces/BP_ChessPiece Object Reference"))
  (set `self.OccupantReference` Piece)
  (return))

(fn `SetPlayerControllerReference`
  (`/Engine/EditorBlueprintResources/StandardMacros.IsValid` (`self.PlayerControllerReference`)
    (:`Is Valid`
      _)
    (:`Is Not Valid`
      (set `self.PlayerControllerReference` (cast `/Game/Chess/Core/Engine/BP_PlayerController_Core` (`GameplayStatics.GetPlayerController` 0) :!pure true))))
  (return))

(fn `SetSquareColor`
  (switch `/Game/Chess/Core/Engine/EColor` (`self.Color`)
    (:`NewEnumerator0`
      (`PrimitiveComponent.SetMaterial` (`self.StaticMesh_Square`) 0 (`self.SquareLightColor`)))
    (:`NewEnumerator1`
      (`PrimitiveComponent.SetMaterial` (`self.StaticMesh_Square`) 0 (`self.SquareDarkColor`))))
  (return))

(fn `UnhighlightMarker`
  (`|ExecutionSequence`
    (:`then_0`
      (set `self.bAttackable` false)
      (set `self.bSelected` false)
      (set `self.bHighlighted` false))
    (:`then_1`
      (`self.SetMarkerColor`)
      (return))))

(fn `UnselectMarker`
  (set `self.bSelected` false)
  (`self.SetMarkerColor`)
  (return))

(fn `UserConstructionScript`
  (`self.SetSquareColor`))